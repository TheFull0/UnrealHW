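; Base weapon component that handles firing and magazine ammo for the actor passed to it through Instantiate.
; Shoot spawns a BP_BaseBullet at that parent's transform, passes it BulletInfo with a zero direction and decrements the magazine, or calls NeedReload when empty.
; Reload pools magazine and reserve ammo to refill the magazine.
; When the pool is short, it loads the remainder only if the magazine is non-empty, otherwise calling NoMoreBullets.
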(event EventBeginPlay)

(event EventTick
  (params (DeltaSeconds :type Float%20%28single-precision%29)))

(event EventShoot
  ;[0.15 0.15 0.15 0.5] Parent Validity Check
  (if (Utilities|IsValid (Variables|Default|GetParent))
    ;[0.15 0.15 0.15 0.5] Bullet Amount Check
    (if (> (Variables|Default|GetCurrentAmmoInMag) 0)
      ;[0.15 0.15 0.15 0.5] Create a Bullet
      (bind _returnvalue (Game|SpawnActorfromClass "/Game/BluePrints/Bullet/BP_BaseBullet.BP_BaseBullet_C" (Transformation|GetActorTransform (Variables|Default|GetParent)) "Undefined" "MultiplyWithRoot" 0 0))
      ;[0.15 0.15 0.15 0.5] Give the Bullet Info
      (Default|SetBulletInfoandShoot _returnvalue (Variables|Default|GetBulletInfo) "0, 0, 0")
      (Variables|Default|SetCurrentAmmoInMag (- (Variables|Default|GetCurrentAmmoInMag) 1))
      (else
        (Default|CallNeedReload)))
    (else
      (Utilities|Debugging|RaiseScriptError "Weapon is not instantiated"))))

(event EventInstantiate
  (params (Parent :type Actor%20Object%20Reference))
  ;[0.15 0.15 0.15 0.5] Set the Controlling Parent for Later Computations and Check Validity
  (if (Utilities|IsValid Parent)
    (Variables|Default|SetParent Parent)
    (else
      (Utilities|Debugging|RaiseScriptError "Parent sent for instantiation is Invalid"))))

(fn Reload
  ;[0.15 0.15 0.15 0.5] Addition of Current and Overall Ammo
  (bind _output_get (Variables|Default|SetOverAllCurrentAmmo (+ (Variables|Default|GetCurrentAmmoInMag) (Variables|Default|GetOverAllCurrentAmmo))))
  ;[0.15 0.15 0.15 0.5] Check Sufficient for Full Amount
  (if (>= _output_get (Variables|Default|GetMaxAmmoPerMag))
    ;[0.15 0.15 0.15 0.5] Reload and Reduce from Current
    (Variables|Default|SetCurrentAmmoInMag (Variables|Default|GetMaxAmmoPerMag))
    (Variables|Default|SetOverAllCurrentAmmo (- (Variables|Default|GetOverAllCurrentAmmo) (Variables|Default|GetMaxAmmoPerMag)))
    (else
      ;[0.15 0.15 0.15 0.5] Check if More Than 0
      (if (> (Variables|Default|GetCurrentAmmoInMag) 0)
        ;[0.15 0.15 0.15 0.5] Unload it All to Magazine and Set to 0
        (Variables|Default|SetCurrentAmmoInMag (Variables|Default|GetOverAllCurrentAmmo))
        (Variables|Default|SetOverAllCurrentAmmo 0)
        (else
          (Default|CallNoMoreBullets))))))