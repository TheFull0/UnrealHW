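; Base weapon Blueprint that fires bullets for an owning Parent and tracks magazine and reserve ammo.
; Once given a Parent, Shoot spawns a BP_BaseBullet at its transform, passes BulletInfo with a zero direction, and decrements the magazine, or calls NeedReload when empty.
; Reload pools magazine and reserve ammo to refill the magazine.
; When short of a full magazine, it checks the old magazine count, not the pool, before loading the remainder or calling NoMoreBullets.
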(event Custom|Shoot
  ;[1 1 1] Parent Validity Check
  (if (Utilities|IsValid (Variables|Default|GetParent))
    ;[1 1 1] Bullet Amount Check
    (if (> (Variables|Default|GetCurrentAmmoInMag) 0)
      ;[1 1 1] Create a Bullet
      (bind _returnvalue (Game|SpawnActorfromClass "/Game/BluePrints/Bullet/BP_BaseBullet.BP_BaseBullet_C" (Transformation|GetActorTransform (Variables|Default|GetParent)) "Undefined" "MultiplyWithRoot" 0 0))
      ;[1 1 1] Give the Bullet Info
      (Default|SetBulletInfoandShoot _returnvalue (Variables|Default|GetBulletInfo) "0, 0, 0")
      (Variables|Default|SetCurrentAmmoInMag (- (Variables|Default|GetCurrentAmmoInMag) 1))
      (else
        (Default|CallNeedReload)))
    (else
      (Utilities|Debugging|RaiseScriptError "Weapon is not instantiated"))))

(event Custom|instantiate_1
  (params (Parent :type Actor%20Object%20Reference))
  ;[1 1 1] Set the Controlling Parent for Later Computations and Check Validity
  (if (Utilities|IsValid Parent)
    (Variables|Default|SetParent Parent)
    (else
      (Utilities|Debugging|RaiseScriptError "Parent sent for instantiation is Invalid"))))

(event EventBeginPlay)

(event EventTick
  (params (DeltaSeconds :type Float%20%28single-precision%29)))

(fn Reload
  ;[1 1 1] Addition of Current and Overall Ammo
  (bind _output_get (Variables|Default|SetOverAllCurrentAmmo (+ (Variables|Default|GetCurrentAmmoInMag) (Variables|Default|GetOverAllCurrentAmmo))))
  ;[1 1 1] Check Sufficient for Full Amount
  (if (>= _output_get (Variables|Default|GetMaxAmmoPerMag))
    ;[1 1 1] Reload and Reduce from Current
    (Variables|Default|SetCurrentAmmoInMag (Variables|Default|GetMaxAmmoPerMag))
    (Variables|Default|SetOverAllCurrentAmmo (- (Variables|Default|GetOverAllCurrentAmmo) (Variables|Default|GetMaxAmmoPerMag)))
    (else
      ;[1 1 1] Check if More Than 0
      (if (> (Variables|Default|GetCurrentAmmoInMag) 0)
        ;[1 1 1] Unload it All to Magazine and Set to 0
        (Variables|Default|SetCurrentAmmoInMag (Variables|Default|GetOverAllCurrentAmmo))
        (Variables|Default|SetOverAllCurrentAmmo 0)
        (else
          (Default|CallNoMoreBullets))))))