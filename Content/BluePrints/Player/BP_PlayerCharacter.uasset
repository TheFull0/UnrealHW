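; Player character Blueprint that handles weapon use, swapping, reloading and pickups, and drives the ammo and game-over UI.
; On BeginPlay it unequips every placed weapon actor, registers itself as their user, and maps them by weapon type through interfaces.
; Weapon pickups unlock and equip the mapped actor, while ammo pickups fill the first owned weapon of matching type, returning leftovers.
; Shots aim along actor forward; the line-trace aiming is unused.
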(event EventBeginPlay
  (bind _outactors (Actor|GetAllActorsOfClass "/Game/BluePrints/Weapons/BP_WeaponBaseClass.BP_WeaponBaseClass_C"))
  ;[1 1 1] Input All Weapon Actors Into a Map With WeaponType as Key
  (for _array_element _outactors
    (bind _asiweapon (Utilities|Casting|CastToIWeapon _array_element))
    (Default|Unequipped _asiweapon)
    (bind _asiweapon_user (Utilities|Casting|CastToIWeaponUser self))
    (Default|SetWeaponUserParent _asiweapon _asiweapon_user)
    (bind _weapontype (Default|GetWeaponType _asiweapon))
    (Utilities|Map|Add (Variables|Default|GetIWeaponTypeMap) _weapontype _asiweapon))
  (bind _returnvalue (UserInterface|CreateWidget "/Game/UI/Ammo_Display_Widget.Ammo_Display_Widget_C"))
  (bind _output_get (Variables|Default|SetUI _returnvalue))
  (UserInterface|Viewport|AddtoViewport _output_get 0))

(event Collision|EventActorBeginOverlap
  (params (OtherActor :type Actor%20Object%20Reference)))

(event EventTick
  (params (DeltaSeconds :type Float%20%28single-precision%29)))

(event EventStartUse
  ;[1 1 1] Shooting
  (if (Variables|Default|GetHasWeapon)
    (Default|StartShoot (Variables|Default|GetEquippedWeapon))))

(event EventReload
  ;[1 1 1] Reload
  (if (Variables|Default|GetHasWeapon)
    (Default|Reload (Variables|Default|GetEquippedWeapon))))

(event EventSwapWeapon
  (bind _pickedupweaponlist (Variables|Default|GetPickedUpWeaponList))
  (bind _returnvalue (Utilities|Array|Length _pickedupweaponlist))
  ;[1 1 1] Check if posses any weapon and swap it out if more thatn 1 weapon
  (if (Variables|Default|GetHasWeapon)
    (if (> _returnvalue 1)
      (Default|Unequipped (Utilities|Array|Get(acopy) (Variables|Default|GetPickedUpWeaponList) (Variables|Default|GetEquippedWeaponIndex)))
      ;[1 1 1] iterate list to next weapon
      (bind _result (Math|Integer|IncrementInt (Variables|Default|GetEquippedWeaponIndex))
        (:%20%20
          (bind _returnvalue_2 (Math|Integer|%(Integer) _result _returnvalue))
          (bind _output_get (Variables|Default|SetEquippedWeaponIndex _returnvalue_2))
          (Default|Equipped (Utilities|Array|Get(acopy) (Variables|Default|GetPickedUpWeaponList) _output_get))
          (Variables|Default|SetEquippedWeapon (Utilities|Array|Get(acopy) (Variables|Default|GetPickedUpWeaponList) _output_get)))))))

(event EventStopUse
  ;[1 1 1] Shooting
  (if (Variables|Default|GetHasWeapon)
    (Default|StopShoot (Variables|Default|GetEquippedWeapon))))

(event EventNotifyOverlapwithPickUp
  (params (PickableObj :type BP%20Pick%20Up%20Base%20Object%20Reference))
  (bind _asbp_ammo_pickup_base (Utilities|Casting|CastToBP_AmmoPickupBase PickableObj)
    (:then
      (if (Variables|Default|GetHasWeapon)
        ;[1 1 1] iterate all equipped weapons and add ammo to first found that uses ammo type
        (bind _array_element (Utilities|Array|ForEachLoopwithBreak (Variables|Default|GetPickedUpWeaponList) :!label _label)
          (:LoopBody
            (bind _ammotype (Default|GetAmmoType _array_element))
            (if (Utilities|Enum|Equal(Enum) _ammotype (Variables|/Game/BluePrints/PickUps/BP_AmmoPickupBase.BP_AmmoPickupBase_C|GetAmmoType _asbp_ammo_pickup_base))
              (bind (_cantakeall _leftover) (Default|AddAmmo _array_element (Variables|/Game/BluePrints/PickUps/BP_AmmoPickupBase.BP_AmmoPickupBase_C|GetAmmoAmount _asbp_ammo_pickup_base)))
              ;[1 1 1] send back leftover ammo that didnt fit in the mag
              (if _cantakeall
                (Default|WasPickedUp _asbp_ammo_pickup_base)
                (goto _label Break)
                (else
                  (Default|SetLeftovers _asbp_ammo_pickup_base _leftover)
                  (goto _label Break))))))))
    (:CastFailed
      (bind _asbp_weapon_pick_up_base (Utilities|Casting|CastToBP_WeaponPickUpBase PickableObj))
      ;[1 1 1] get the coresponding class from the array and check if you already posses it
      (bind (_value _returnvalue) (Utilities|Map|Find (Variables|Default|GetIWeaponTypeMap) (Variables|/Game/BluePrints/PickUps/BP_WeaponPickUpBase.BP_WeaponPickUpBase_C|GetWeapon%20Type _asbp_weapon_pick_up_base)))
      (if _returnvalue
        (bind _returnvalue_2 (Utilities|Array|ContainsItem (Variables|Default|GetPickedUpWeaponList) _value))
        (if (not _returnvalue_2)
          ;[1 1 1] Add the weapon to possesion list and swap to it
          (Default|WasPickedUp PickableObj)
          (CallFunction|UnequipLast)
          (bind _returnvalue_3 (Utilities|Array|Add (Variables|Default|GetPickedUpWeaponList) _value))
          (Variables|Default|SetEquippedWeaponIndex _returnvalue_3)
          (Default|Equipped _value)
          (Variables|Default|SetEquippedWeapon _value)
          (Variables|Default|SetHasWeapon true))))))

(fn ConstructionScript)

(fn UnequipLast
  (if (Variables|Default|GetHasWeapon)
    (Default|Unequipped (Variables|Default|GetEquippedWeapon))))

(fn Lose
  (Default|CallGameOver (Variables|Default|GetUI) false))

(fn Win
  (Default|CallGameOver (Variables|Default|GetUI) true))

(fn BulletWasShotUpdateUI
  (params (current :type Integer) (max :type Integer))
  (Default|CallUpdateAmmoText (Variables|Default|GetUI) current max)
  (return))

(fn GetShootingVector
  (return (Transformation|GetActorForwardVector)))