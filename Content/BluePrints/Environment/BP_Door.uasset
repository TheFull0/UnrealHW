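; A two-panel sliding door that opens when the player character overlaps it and closes when the player leaves.
; Entering swaps both panels to the laser pointer material instance and plays the open timeline, and leaving restores the base material and plays the close timeline.
; Each timeline stops the other, then lerps the panels from their current positions toward open or origin marker components, so reversing mid-motion continues from where they are.
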(event EventBeginPlay)

(event Collision|EventActorBeginOverlap
  (params (OtherActor :type Actor%20Object%20Reference))
  (bind _asbp_player_character (Utilities|Casting|CastToBP_PlayerCharacter OtherActor))
  (Utilities|IsValid _asbp_player_character
    (:Is%20Valid
      (Rendering|Material|SetMaterial (Variables|Default|GetLeft%20Panel) 0 "/Engine/VREditor/LaserPointer/LaserPointerMaterial_Inst.LaserPointerMaterial_Inst")
      (Rendering|Material|SetMaterial (Variables|Default|GetRight%20Panel) 0 "/Engine/VREditor/LaserPointer/LaserPointerMaterial_Inst.LaserPointerMaterial_Inst")
      (Utilities|FlowControl|Sequence
        (:then_0
          ;[1 1 1] Transition to non aimed camera
          (bind _doormove (Timeline|TL_DoorClose Stop)
            (:Update
              (Utilities|FlowControl|Sequence
                (:then_0
                  (Transformation|SetWorldLocation (Variables|Default|GetLeft%20Panel) (Math|Vector|Lerp(Vector) (Transformation|GetWorldLocation (Variables|Default|GetLeft%20Panel)) (Transformation|GetWorldLocation (Variables|Default|GetOriginLeft)) _doormove) false false))
                (:then_1
                  (Transformation|SetWorldLocation (Variables|Default|GetRight%20Panel) (Math|Vector|Lerp(Vector) (Transformation|GetWorldLocation (Variables|Default|GetRight%20Panel)) (Transformation|GetWorldLocation (Variables|Default|GetOriginRight)) _doormove) false false))))))
        (:then_1
          ;[1 1 1] Transition to aimed camera
          (bind _doormove_2 (Timeline|TL_DoorOpen PlayFromStart)
            (:Update
              (Utilities|FlowControl|Sequence
                (:then_0
                  (Transformation|SetWorldLocation (Variables|Default|GetLeft%20Panel) (Math|Vector|Lerp(Vector) (Transformation|GetWorldLocation (Variables|Default|GetLeft%20Panel)) (Transformation|GetWorldLocation (Variables|Default|GetOpenLeft)) _doormove_2) false false))
                (:then_1
                  (Transformation|SetWorldLocation (Variables|Default|GetRight%20Panel) (Math|Vector|Lerp(Vector) (Transformation|GetWorldLocation (Variables|Default|GetRight%20Panel)) (Transformation|GetWorldLocation (Variables|Default|GetOpenRight)) _doormove_2) false false))))))))))

(event EventTick
  (params (DeltaSeconds :type Float%20%28single-precision%29)))

(event Collision|EventActorEndOverlap
  (params (OtherActor :type Actor%20Object%20Reference))
  (bind _asbp_player_character (Utilities|Casting|CastToBP_PlayerCharacter OtherActor))
  (Utilities|IsValid _asbp_player_character
    (:Is%20Valid
      (Rendering|Material|SetMaterial (Variables|Default|GetLeft%20Panel) 0 "/Engine/VREditor/LaserPointer/LaserPointerMaterial.LaserPointerMaterial")
      (Rendering|Material|SetMaterial (Variables|Default|GetRight%20Panel) 0 "/Engine/VREditor/LaserPointer/LaserPointerMaterial.LaserPointerMaterial")
      (Utilities|FlowControl|Sequence
        (:then_0
          ;[1 1 1] Transition to aimed camera
          (bind _doormove (Timeline|TL_DoorOpen Stop)
            (:Update
              (Utilities|FlowControl|Sequence
                (:then_0
                  (Transformation|SetWorldLocation (Variables|Default|GetLeft%20Panel) (Math|Vector|Lerp(Vector) (Transformation|GetWorldLocation (Variables|Default|GetLeft%20Panel)) (Transformation|GetWorldLocation (Variables|Default|GetOpenLeft)) _doormove) false false))
                (:then_1
                  (Transformation|SetWorldLocation (Variables|Default|GetRight%20Panel) (Math|Vector|Lerp(Vector) (Transformation|GetWorldLocation (Variables|Default|GetRight%20Panel)) (Transformation|GetWorldLocation (Variables|Default|GetOpenRight)) _doormove) false false))))))
        (:then_1
          ;[1 1 1] Transition to non aimed camera
          (bind _doormove_2 (Timeline|TL_DoorClose PlayFromStart)
            (:Update
              (Utilities|FlowControl|Sequence
                (:then_0
                  (Transformation|SetWorldLocation (Variables|Default|GetLeft%20Panel) (Math|Vector|Lerp(Vector) (Transformation|GetWorldLocation (Variables|Default|GetLeft%20Panel)) (Transformation|GetWorldLocation (Variables|Default|GetOriginLeft)) _doormove_2) false false))
                (:then_1
                  (Transformation|SetWorldLocation (Variables|Default|GetRight%20Panel) (Math|Vector|Lerp(Vector) (Transformation|GetWorldLocation (Variables|Default|GetRight%20Panel)) (Transformation|GetWorldLocation (Variables|Default|GetOriginRight)) _doormove_2) false false))))))))))

(fn ConstructionScript)