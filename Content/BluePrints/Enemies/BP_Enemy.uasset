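; BP_Enemy is an enemy Blueprint that tracks hit points and handles its own death.
; HP starts at MaxHP, DealDamage subtracts from it, and at zero or below it calls EnemyDeath before destroying the actor.
; ChaseTick is an empty stub.
; CheckTragetDistanceInRange is a placeholder that compares the actor's location with itself against zero, so it always returns false.
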(event EventBeginPlay
  (Variables|Default|SetHP (Variables|Default|GetMaxHP)))

(event EventDealDamage
  (params (DamageAmount :type Integer))
  (bind _output_get (Variables|Default|SetHP (- (Variables|Default|GetHP) DamageAmount)))
  (if (<= _output_get 0)
    (Default|CallEnemyDeath)
    (Actor|DestroyActor)))

(fn ConstructionScript)

(fn ChaseTick
  (params (delta%20time :type Float%20%28double-precision%29)))

(fn CheckTragetDistanceinRange
  (return (< (Math|Vector|Distance(Vector) (Transformation|GetActorLocation) (Transformation|GetActorLocation)) 0.0)))