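; Game mode for a kill-all-enemies level: the player wins when every BP_Enemy dies and loses on touching one.
; BeginPlay binds each enemy's death and overlap events, which update the count and alive flag and print the result.
; Random ammo pickups spawn inside that enemy loop, re-rolling type separately from the branch that sets amount.
; It also hands PatrolPoint-tagged actors to every BP_EnemyAI as patrol points.
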(event Custom|OnPlayerOverlapWithEnemy_Event
  (Variables|Default|SetPlayerAlive false)
  (Development|PrintString "Player Was Touched To Death By Enemy!!!!!!!!!" true true "(R=1.000000,G=0.000000,B=0.000000,A=1.000000)" 3e+01 "PlayerDead"))

(event Custom|OnEnemyDeath
  ;[1 1 1] enemy death event
  (bind _result (Math|Integer|DecrementInt (Variables|Default|GetEnemyAmount))
    (:%20%20
      (bind _output_get (Variables|Default|SetEnemyAmount _result))
      (if (and (<= _output_get 0) (Variables|Default|GetPlayerAlive))
        (Development|PrintString "Player Won and Killed All Targets!!!!" true true "(R=0.163751,G=1.000000,B=0.004503,A=1.000000)" 3e+01 "Win")))))

(event EventBeginPlay
  (bind _returnvalue (Math|Random|RandomInteger 2))
  (bind _returnvalue_2 (Math|Conversions|ToByte(Integer) _returnvalue))
  (bind _returnvalue_3 (Utilities|Enum|ByteToEnumE_AmmoType _returnvalue_2))
  (bind _outactors (Actor|GetAllActorsOfClass "/Game/BluePrints/Enemies/BP_Enemy.BP_Enemy_C"))
  (Variables|Default|SetEnemyAmount (Utilities|Array|Length _outactors))
  (for _array_element _outactors
    (EventDispatchers|BindEventtoEnemyDeath _array_element (delegate Custom|OnEnemyDeath))
    (EventDispatchers|BindEventtoPlayerOverlap _array_element (delegate Custom|OnPlayerOverlapWithEnemy_Event))
    (while (> (Variables|Default|GetAmmoToCreate) 0)
      ;[1 1 1] randomize ammo type
      (switch Utilities|FlowControl|Switch|SwitchonE_AmmoType _returnvalue_3
        (:NewEnumerator0
          ;[1 1 1] grenade ammo
          (Game|SpawnActorfromClass "/Game/BluePrints/PickUps/BP_AmmoPickupBase.BP_AmmoPickupBase_C" (Math|Transform|MakeTransform (Math|Vector|MakeVector (Math|Conversions|ToFloat(Integer) (Math|Random|RandomIntegerinRange 0 1000)) (Math|Conversions|ToFloat(Integer) (Math|Random|RandomIntegerinRange 0 1000)) 1e+01) "0, 0, 0" "1.000000,1.000000,1.000000") "AlwaysSpawn" "MultiplyWithRoot" 0 (Math|Random|RandomIntegerinRange 5 10) _returnvalue_3 0))
        (:NewEnumerator1
          ;[1 1 1] Medium ammo
          (Game|SpawnActorfromClass "/Game/BluePrints/PickUps/BP_AmmoPickupBase.BP_AmmoPickupBase_C" (Math|Transform|MakeTransform (Math|Vector|MakeVector (Math|Conversions|ToFloat(Integer) (Math|Random|RandomIntegerinRange 0 1000)) (Math|Conversions|ToFloat(Integer) (Math|Random|RandomIntegerinRange 0 1000)) 1e+01) "0, 0, 0" "1.000000,1.000000,1.000000") "Undefined" "MultiplyWithRoot" 0 (Math|Random|RandomIntegerinRange 10 20) _returnvalue_3 0)))
      ;[1 1 1] decrease spawning amout
      (bind _result (Math|Integer|DecrementInt (Variables|Default|GetAmmoToCreate))
        (:%20%20
          (Variables|Default|SetAmmoToCreate _result)))))
  (bind _outactors_2 (Actor|GetAllActorswithTag "PatrolPoint"))
  (bind _outactors_3 (Actor|GetAllActorsOfClass "/Game/BluePrints/Enemies/BP_EnemyAI.BP_EnemyAI_C"))
  (for _array_element_2 _outactors_3
    (Default|SetPatrolPoints _array_element_2 _outactors_2)))

(event EventTick
  (params (DeltaSeconds :type Float%20%28single-precision%29)))

(fn ConstructionScript)